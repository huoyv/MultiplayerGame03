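; BP_Target is a replicated shootable target for a multiplayer game that is randomly either Good or Bad.
; The server picks the state on BeginPlay, and its RepNotify swaps the cone's material to match, as the construction script does.
; When damaged by a player, it updates that player's room PlayerState score, penalizing Good and rewarding Bad, then destroys the damage causer and itself.
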(event EventBeginPlay
  (Networking|SwitchHasAuthority
    (:Authority
      (CallFunction|RandomSwitchState))))

(event Game|Damage|EventAnyDamage
  (params (Damage :type Float%20%28single-precision%29) (DamageType :type Damage%20Type%20Object%20Reference) (InstigatedBy :type Controller%20Object%20Reference) (DamageCauser :type Actor%20Object%20Reference))
  (bind _as玩家控制器 (Utilities|Casting|CastToPlayerController InstigatedBy))
  (bind _asbp_room_player_state (Utilities|Casting|CastToBP_RoomPlayerState (Variables|/Script/Engine.Controller|GetPlayerState _as玩家控制器))
    (:then
      (Default|UpdateScore _asbp_room_player_state (Utilities|Select :Index (Variables|Default|GetTargetState) :NewEnumerator0 -2.0 :NewEnumerator1 1.0)))
    (:CastFailed
      _))
  (Actor|DestroyActor DamageCauser)
  (Actor|DestroyActor))

(fn ConstructionScript
  (Rendering|Material|SetMaterial (Variables|Default|GetCone) 0 (Utilities|Select :Index (Variables|Default|GetTargetState) :NewEnumerator0 "/Game/MultiplayerGame/Blueprints/Gameplay/Target/MI_GoodTargetMaterial_Inst.MI_GoodTargetMaterial_Inst" :NewEnumerator1 "/Game/MultiplayerGame/Blueprints/Gameplay/Target/MI_BadTargetMaterial_Inst.MI_BadTargetMaterial_Inst")))

(fn OnRepTargetState
  (Rendering|Material|SetMaterial (Variables|Default|GetCone) 0 (Utilities|Select :Index (Variables|Default|GetTargetState) :NewEnumerator0 "/Game/MultiplayerGame/Blueprints/Gameplay/Target/MI_GoodTargetMaterial_Inst.MI_GoodTargetMaterial_Inst" :NewEnumerator1 "/Game/MultiplayerGame/Blueprints/Gameplay/Target/MI_BadTargetMaterial_Inst.MI_BadTargetMaterial_Inst")))

(fn RandomSwitchState
  (Variables|Default|SetTargetState (select (>= (Math|Random|RandomFloatinRange 0.0 1.0) 0.5) "NewEnumerator1" "NewEnumerator0")))