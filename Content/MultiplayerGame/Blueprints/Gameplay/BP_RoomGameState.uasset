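; BP_RoomGameState is a game state that runs the countdown timer for a room's match.
; SettTimer stores the map time as the maximum and remaining time and starts the countdown.
; Tick reduces the remaining time, clamped at zero, while the game is running.
; At zero, a DoOnce and an authority check let only the server tell BP_RoomGameMode to call GameOver, a single time.
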(event Custom|SettTimer
  (params (MapTime :type Float%20%28single-precision%29))
  (bind _output_get (Variables|Default|SetMaxTime MapTime))
  (Variables|Default|SetTimeLeft _output_get)
  (Variables|Default|SetGameRunning true))

(event EventTick
  (params (DeltaSeconds :type Float%20%28single-precision%29))
  (if (Variables|Default|GetGameRunning)
    (bind _output_get (Variables|Default|SetTimeLeft (Math|Float|Clamp(Float) (- (Variables|Default|GetTimeLeft) DeltaSeconds) 0.0 (Variables|Default|GetMaxTime))))
    (if (== _output_get 0.0)
      (Utilities|FlowControl|DoOnce false
        (:Completed
          (Networking|SwitchHasAuthority
            (:Authority
              (bind _asbp_room_game_mode (Utilities|Casting|CastToBP_RoomGameMode (Game|GetGameMode)))
              (Default|GameOver _asbp_room_game_mode))))))))

(fn ConstructionScript)